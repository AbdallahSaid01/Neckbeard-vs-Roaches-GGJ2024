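; BP_Cockroach is an enemy pawn that walks to the sandwich and damages it on contact.
; BeginPlay finds BP_Sandwich and sends the cockroach toward it with AIMoveTo.
; Overlapping the sandwich's sphere component calls DamageSandwich, then destroys the cockroach after a short delay.
; Incoming damage lowers clamped Health, destroying it at zero, and a separate function can halt and deactivate its movement.
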(event `self.ReceiveBeginPlay`
  (bind _returnvalue (`GameplayStatics.GetActorOfClass` "/Game/Game/Assets/Enemy/Blueprints/BP_Sandwich.BP_Sandwich_C"))
  (`|AIMoveTo` self (0.0 0.0 0.0) _returnvalue))

(event `self.ReceiveAnyDamage`
  (params (Damage :type "Float (single-precision)") (DamageType :type "DamageType Object Reference") (InstigatedBy :type "Controller Object Reference") (DamageCauser :type "Actor Object Reference"))
  (if true
    (bind _output_get (`self.DecreaseHealth` Damage))
    (if (== _output_get 0.0)
      (`KismetSystemLibrary.Delay` 0.2)
      (`self.K2_DestroyActor`))))

(event `self.CapsuleComponent.OnComponentBeginOverlap`
  (params (OverlappedComponent :type "PrimitiveComponent Object Reference") (OtherActor :type "Actor Object Reference") (OtherComp :type "PrimitiveComponent Object Reference") (OtherBodyIndex :type Integer) (bFromSweep :type Boolean) (SweepResult :type "HitResult Structure (by ref)"))
  (bind _asbp_sandwich (cast `/Game/Game/Assets/Enemy/Blueprints/BP_Sandwich` OtherActor))
  (if (== OtherComp (`self.GetComponentByClass` _asbp_sandwich "/Script/Engine.SphereComponent"))
    (`/Game/Game/Assets/Enemy/Blueprints/BP_Sandwich.Damage Sandwich` _asbp_sandwich (`self.Damage Per Hit`))
    (`KismetSystemLibrary.Delay` 0.2)
    (`self.K2_DestroyActor`)))

(fn `Deactivate AI Movement`
  (bind _charactermovement (`self.CharacterMovement`))
  (`MovementComponent.StopMovementImmediately` _charactermovement)
  (`ActorComponent.Deactivate` _charactermovement))

(fn `DecreaseHealth`
  (params (`Damage Amount` :type "Float (double-precision)"))
  (returns (Output_Get :type "Float (double-precision)"))
  (bind _output_get (set `self.Health` (`KismetMathLibrary.FClamp` (- (`self.Health`) `Damage Amount`) 0.0 100.0)))
  (if (== _output_get 0.0)
    (`self.K2_DestroyActor`))
  (return _output_get))

(fn `UserConstructionScript`)