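; BP_Sandwich is the player's sandwich, a health-bearing objective whose loss ends the level.
; DamageSandwich subtracts damage from a clamped Health value and, while any remains, passes the unscaled value to the health progress bar in every W_PlayerHUD widget, then returns it.
; At zero it prints a red "eaten" message and has BP_FirstPersonGameMode switch to MainMenu.
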(fn `Damage Sandwich`
  (params (`Damage Amount` :type "Float (double-precision)"))
  (returns (Health :type "Float (double-precision)"))
  (bind _output_get (set `self.Health` (`KismetMathLibrary.FClamp` (- (`self.Health`) `Damage Amount`) 0.0 100.0)))
  (if (== _output_get 0.0)
    (`KismetSystemLibrary.PrintString` "YOUR SANDWICH HAS BEEN EATEN" true true (struct :`R` 1.0 :`G` 0.009271 :`A` 1.0))
    (bind _asbp_first_person_game_mode (cast `/Game/FirstPersonTemplate/FirstPerson/Blueprints/BP_FirstPersonGameMode` (`GameplayStatics.GetGameMode`)))
    (`/Game/FirstPersonTemplate/FirstPerson/Blueprints/BP_FirstPersonGameMode.Switch Level` _asbp_first_person_game_mode "MainMenu")
    (else
      (bind _foundwidgets (`WidgetBlueprintLibrary.GetAllWidgetsOfClass` "/Game/Game/Blueprints/WidgetBlueprints/W_PlayerHUD.W_PlayerHUD_C" false))
      (for _array_element _foundwidgets
        (`ProgressBar.SetPercent` (`/Game/Game/Blueprints/WidgetBlueprints/W_PlayerHUD.ProgressBar_PlayerHealth` _array_element) _output_get))
      (return _output_get))))

(fn `UserConstructionScript`)